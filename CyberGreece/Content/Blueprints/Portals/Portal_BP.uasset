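; Linked portal actor that shows the view through its partner and teleports the first-person player between the two.
; While active, it moves the linked portal's scene capture to the player's mirrored view, rendering into a viewport-sized render target on its plane material.
; A clip plane trims the capture and the plane shifts to avoid near-camera clipping.
; A plane-crossing test triggers the teleport, remapping transform, control rotation and velocity with a camera cut.
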(event EventBeginPlay
  (bind _returnvalue (Viewport|GetViewportSize))
  (Utilities|FlowControl|Delay 0.001)
  (Components|Tick|SetTickGroup "TG_PostUpdateWork")
  (bind _returnvalue_2 (Rendering|Material|CreateDynamicMaterialInstance "/Game/Blueprints/Portals/Portal_M.Portal_M" "" "None" :!class /Script/Engine.KismetMaterialLibrary))
  (bind _output_get (Variables|Default|SetPortal_MAT _returnvalue_2))
  (Rendering|Material|SetMaterial (Variables|Default|GetPortal%20Plane) 0 _output_get)
  (bind _returnvalue_3 (Rendering|CreateRenderTarget2D (Math|Float|Truncate (.x _returnvalue)) (Math|Float|Truncate (.y _returnvalue)) "RTF_RGBA16f"))
  (bind _output_get_2 (Variables|Default|SetPortal_RT _returnvalue_3))
  (Rendering|Material|SetTextureParameterValue (Variables|Default|GetPortal_MAT) "Texture" _output_get_2)
  (Variables|/Script/Engine.SceneCaptureComponent2D|SetTextureTarget (Variables|Portal_BP_C|GetPortal%20Camera (Variables|Default|GetLinked%20Portal)) (Variables|Default|GetPortal_RT))
  (CallFunction|SetClipPlanes)
  (bind _returnvalue_4 (Actor|GetActorOfClass "/Game/FirstPerson/Blueprints/BP_FirstPersonCharacter.BP_FirstPersonCharacter_C"))
  (Variables|Default|SetPlayerCharacter _returnvalue_4))

(event Collision|EventActorBeginOverlap
  (params (OtherActor :type Actor%20Object%20Reference)))

(event EventTick
  (params (DeltaSeconds :type Float%20%28single-precision%29))
  (if (Variables|Default|GetisActive)
    (Rendering|SetVisibility (Variables|Default|GetPortal%20Plane) true false)
    (CallFunction|UpdateSceneCapture)
    (CallFunction|PreventPlaneClipping)
    (CallFunction|CheckViewportSize)
    (CallFunction|ShouldTeleport)
    (else
      (Rendering|SetVisibility (Variables|Default|GetPortal%20Plane) false false))))

(fn ConstructionScript)

(fn UpdateSceneCapture
  (bind _returnvalue (Transformation|GetActorTransform))
  (bind _returnvalue_2 (Transformation|GetActorTransform))
  (bind _returnvalue_3 (Game|GetPlayerCameraManager 0))
  (bind _linked_portal (Variables|Default|GetLinked%20Portal))
  (bind (_location _rotation _scale) (Math|Transform|BreakTransform _returnvalue))
  (bind _returnvalue_4 (Transformation|GetActorTransform _linked_portal))
  (bind _transformcomponent (Variables|/Script/Engine.PlayerCameraManager|GetTransformComponent _returnvalue_3))
  (bind _returnvalue_5 (Transformation|GetWorldRotation _transformcomponent))
  (bind (_x _y _z) (Math|Vector|BreakVector _scale))
  (bind (_x_2 _y_2 _z_2) (Math|Rotator|BreakRotIntoAxes _returnvalue_5))
  (Transformation|SetWorldLocationAndRotation (Variables|Portal_BP_C|GetPortal%20Camera (Variables|Default|GetLinked%20Portal)) (Math|Transform|TransformLocation (Transformation|GetActorTransform (Variables|Default|GetLinked%20Portal)) (Math|Transform|InverseTransformLocation (Math|Transform|MakeTransform _location _rotation (Math|Vector|MakeVector (* _x -1.0) (* _y -1.0) _z)) (Transformation|GetWorldLocation (Variables|/Script/Engine.PlayerCameraManager|GetTransformComponent (Game|GetPlayerCameraManager 0))))) (Math|Rotator|MakeRotationfromAxes (Math|Transform|TransformDirection _returnvalue_4 (Math|Vector|MirrorVectorbyNormal (Math|Vector|MirrorVectorbyNormal (Math|Transform|InverseTransformDirection _returnvalue_2 _x_2) "1.000000,0.000000,0.000000") "0.000000,1.000000,0.000000")) (Math|Transform|TransformDirection _returnvalue_4 (Math|Vector|MirrorVectorbyNormal (Math|Vector|MirrorVectorbyNormal (Math|Transform|InverseTransformDirection _returnvalue_2 _y_2) "1.000000,0.000000,0.000000") "0.000000,1.000000,0.000000")) (Math|Transform|TransformDirection _returnvalue_4 (Math|Vector|MirrorVectorbyNormal (Math|Vector|MirrorVectorbyNormal (Math|Transform|InverseTransformDirection _returnvalue_2 _z_2) "1.000000,0.000000,0.000000") "0.000000,1.000000,0.000000"))) false false))

(fn SetClipPlanes
  (bind _portal_camera (Variables|Default|GetPortal%20Camera))
  (Utilities|IsValid (Variables|Default|GetLinked%20Portal)
    (:Is%20Valid
      (Variables|/Script/Engine.SceneCaptureComponent2D|SetbEnableClipPlane _portal_camera true)
      (Variables|/Script/Engine.SceneCaptureComponent2D|SetClipPlaneBase _portal_camera (+ (Transformation|GetWorldLocation (Variables|Default|GetPortal%20Camera)) (* (Math|Vector|GetForwardVector (Variables|Default|GetForward%20Direction)) -3.0)))
      (Variables|/Script/Engine.SceneCaptureComponent2D|SetClipPlaneNormal _portal_camera (Math|Vector|GetForwardVector (Variables|Default|GetForward%20Direction))))))

(fn CheckViewportSize
  (bind _returnvalue (Viewport|GetViewportSize))
  (bind _returnvalue_2 (Viewport|GetViewportSize))
  (bind _portal_rt (Variables|Default|GetPortal_RT))
  (bind (_x _y) (Math|Vector2D|BreakVector2D _returnvalue))
  (bind (_x_2 _y_2) (Math|Vector2D|BreakVector2D _returnvalue_2))
  (if (not (and (== _x_2 (Variables|/Script/Engine.TextureRenderTarget2D|GetSizeX _portal_rt)) (== _y_2 (Variables|/Script/Engine.TextureRenderTarget2D|GetSizeY _portal_rt))))
    (Rendering|ResizeRenderTarget2D (Variables|Default|GetPortal_RT) (Math|Float|Truncate _x) (Math|Float|Truncate _y))))

(fn ShouldTeleport
  (Utilities|IsValid (Utilities|Array|Get(acopy) (Collision|GetOverlappingActors (Variables|Default|GetPlayer%20Detection) "/Game/FirstPerson/Blueprints/BP_FirstPersonCharacter.BP_FirstPersonCharacter_C" :!class /Script/Engine.PrimitiveComponent))
    (:Is%20Valid
      (bind _return (CallFunction|IsPointCrossingPortal (Transformation|GetWorldLocation (Variables|/Script/Engine.Actor|GetRootComponent (Variables|Default|GetPlayerCharacter))) (Transformation|GetActorLocation) (Math|Vector|GetForwardVector (Variables|Default|GetForward%20Direction))))
      (if _return
        (Development|PrintString "teleport")
        (CallFunction|TeleportCharacter)))))

(fn IsPointCrossingPortal
  (params (Point :type Vector) (PortalLocation :type Vector) (PortalNormal :type Vector))
  (LocalVariables|SetisInFront (>= (Math|Vector|DotProduct PortalNormal (- Point PortalLocation)) 0.0))
  (bind _output_get (LocalVariables|SetportalPlane (Class|KismetMathLibrary|MakePlanefromPointandNormal PortalLocation PortalNormal)))
  (LocalVariables|SetisIntersect (.ReturnValue (Class|KismetMathLibrary|LinePlaneIntersection (Variables|Default|GetLastPosition) Point _output_get)))
  (LocalVariables|SetisCrossing (Math|Boolean|ANDBoolean (LocalVariables|GetisIntersect) (not (LocalVariables|GetisInFront)) (Variables|Default|GetLastInFront)))
  (Variables|Default|SetLastInFront (LocalVariables|GetisInFront))
  (Variables|Default|SetLastPosition Point)
  (return (LocalVariables|GetisCrossing)))

(fn TeleportCharacter
  (bind _returnvalue (Transformation|GetActorTransform))
  (bind _returnvalue_2 (Transformation|GetActorTransform))
  (bind _returnvalue_3 (Transformation|GetActorTransform))
  (bind _returnvalue_4 (Game|GetPlayerController 0))
  (bind _returnvalue_5 (Game|GetPlayerCharacter 0))
  (bind _linked_portal (Variables|Default|GetLinked%20Portal))
  (bind _linked_portal_2 (Variables|Default|GetLinked%20Portal))
  (bind _playercharacter (Variables|Default|GetPlayerCharacter))
  (bind _returnvalue_6 (Transformation|GetActorTransform _linked_portal))
  (bind _returnvalue_7 (Transformation|GetActorRotation _playercharacter))
  (bind (_location _rotation _scale) (Math|Transform|BreakTransform _returnvalue_2))
  (bind _returnvalue_8 (Transformation|GetActorTransform _linked_portal_2))
  (bind _returnvalue_9 (Pawn|GetControlRotation _returnvalue_4 :!class /Script/Engine.Controller))
  (bind _returnvalue_10 (Pawn|GetMovementComponent _returnvalue_5))
  (bind (_x _y _z) (Math|Rotator|GetAxes _returnvalue_9))
  (bind (_x_2 _y_2 _z_2) (Math|Rotator|GetAxes _returnvalue_7))
  (bind _returnvalue_11 (Math|Transform|InverseTransformDirection _returnvalue _z))
  (bind _returnvalue_12 (Math|Transform|InverseTransformDirection _returnvalue _x))
  (bind _returnvalue_13 (Math|Transform|InverseTransformDirection _returnvalue _y))
  (bind _returnvalue_14 (Math|Vector|MirrorVectorbyNormal _returnvalue_11 "1.000000,0.000000,0.000000"))
  (bind _returnvalue_15 (Math|Vector|MirrorVectorbyNormal _returnvalue_12 "1.000000,0.000000,0.000000"))
  (bind _returnvalue_16 (Math|Vector|MirrorVectorbyNormal _returnvalue_13 "1.000000,0.000000,0.000000"))
  (bind _returnvalue_17 (Math|Vector|MirrorVectorbyNormal _returnvalue_14 "0.000000,1.000000,0.000000"))
  (bind _returnvalue_18 (Math|Vector|MirrorVectorbyNormal _returnvalue_15 "0.000000,1.000000,0.000000"))
  (bind _returnvalue_19 (Math|Vector|MirrorVectorbyNormal _returnvalue_16 "0.000000,1.000000,0.000000"))
  (bind _returnvalue_20 (Math|Transform|TransformDirection _returnvalue_6 _returnvalue_17))
  (bind _returnvalue_21 (Math|Transform|TransformDirection _returnvalue_6 _returnvalue_18))
  (bind _returnvalue_22 (Math|Transform|TransformDirection _returnvalue_6 _returnvalue_19))
  (bind _returnvalue_23 (Math|Rotator|MakeRotationfromAxes _returnvalue_21 _returnvalue_22 _returnvalue_20))
  (Transformation|SetActorTransform (Variables|Default|GetPlayerCharacter) (Math|Transform|MakeTransform (Math|Transform|TransformLocation (Transformation|GetActorTransform (Variables|Default|GetLinked%20Portal)) (Math|Transform|InverseTransformLocation (Math|Transform|MakeTransform _location _rotation (Math|Vector|MakeVector (* (.x _scale) -1.0) (* (.y _scale) -1.0) (.z _scale))) (Transformation|GetActorLocation (Variables|Default|GetPlayerCharacter)))) (Math|Rotator|MakeRotationfromAxes (Math|Transform|TransformDirection _returnvalue_8 (Math|Vector|MirrorVectorbyNormal (Math|Vector|MirrorVectorbyNormal (Math|Transform|InverseTransformDirection _returnvalue_3 _x_2) "1.000000,0.000000,0.000000") "0.000000,1.000000,0.000000")) (Math|Transform|TransformDirection _returnvalue_8 (Math|Vector|MirrorVectorbyNormal (Math|Vector|MirrorVectorbyNormal (Math|Transform|InverseTransformDirection _returnvalue_3 _y_2) "1.000000,0.000000,0.000000") "0.000000,1.000000,0.000000")) (Math|Transform|TransformDirection _returnvalue_8 (Math|Vector|MirrorVectorbyNormal (Math|Vector|MirrorVectorbyNormal (Math|Transform|InverseTransformDirection _returnvalue_3 _z_2) "1.000000,0.000000,0.000000") "0.000000,1.000000,0.000000"))) "1.000000,1.000000,1.000000") false true)
  (Pawn|SetControlRotation (Game|GetPlayerController 0) _returnvalue_23)
  (bind _returnvalue_24 (CallFunction|UpdateVelocity (Variables|/Script/Engine.MovementComponent|GetVelocity _returnvalue_10)))
  (Variables|/Script/Engine.MovementComponent|SetVelocity _returnvalue_10 _returnvalue_24)
  (Default|SmoothOrientation (.AsBP%20First%20Person%20Character (Utilities|Casting|CastToBP_FirstPersonCharacter (Game|GetPlayerCharacter 0))) _returnvalue_23)
  (Class|PlayerCameraManager|SetGameCameraCutThisFrame (Game|GetPlayerCameraManager 0)))

(fn UpdateVelocity
  (params (Velocity :type Vector))
  (return (* (Math|Transform|TransformDirection (Transformation|GetActorTransform (Variables|Default|GetLinked%20Portal)) (Math|Vector|MirrorVectorbyNormal (Math|Vector|MirrorVectorbyNormal (Math|Transform|InverseTransformDirection (Transformation|GetActorTransform) (Math|Vector|Normalize Velocity)) "0, 0, 0") "0, 0, 0")) (Math|Vector|VectorLength (Transformation|GetVelocity)))))

(fn PreventPlaneClipping
  (bind _returnvalue (Game|GetPlayerCharacter 0))
  (bind _returnvalue_2 (Transformation|GetActorLocation))
  (bind _forward_direction (Variables|Default|GetForward%20Direction))
  (bind _returnvalue_3 (Math|Vector|GetForwardVector _forward_direction))
  (bind _asbp_first_person_character (Utilities|Casting|CastToBP_FirstPersonCharacter _returnvalue))
  (bind _firstpersoncamera (Variables|/Game/FirstPerson/Blueprints/BP_FirstPersonCharacter.BP_FirstPersonCharacter_C|GetFirstPersonCamera _asbp_first_person_character))
  (bind _returnvalue_4 (Transformation|GetWorldLocation _firstpersoncamera))
  (bind _returnvalue_5 (- _returnvalue_4 _returnvalue_2))
  (bind _returnvalue_6 (Math|Vector|DotProduct _returnvalue_3 _returnvalue_5))
  (if (and (>= _returnvalue_6 -3.0) (<= _returnvalue_6 0.0))
    (Transformation|SetRelativeLocation (Variables|Default|GetPortal%20Plane) "2.000000,0.000000,100.000000" false false)
    (elif (and (>= _returnvalue_6 -3.0) (<= _returnvalue_6 3.0))
      (Transformation|SetRelativeLocation (Variables|Default|GetPortal%20Plane) "-2.000000,0.000000,100.000000" false false)
      (else
        (Transformation|SetRelativeLocation (Variables|Default|GetPortal%20Plane) "0.000000,0.000000,100.000000" false false)))))

(fn DisablePortal
  (Rendering|SetVisibility (Variables|Default|GetDefaultSceneRoot) false false))

(fn EnablePortal
  (Rendering|SetVisibility (Variables|Default|GetDefaultSceneRoot) true false))