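; BP_YarnBall is a save point that lets the first-person character save when nearby.
; Overlapping its collision sphere, sized from InteractDistance in the construction script, sets the player's CanSave flag, registers itself as NearestBall and shows a save-game widget.
; Leaving the sphere clears CanSave and removes the widget.
; Tick bobs the Sphere component vertically with a time-based sine offset.
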(event OnComponentBeginOverlap(CollisionSphere)
  (params (OverlappedComponent :type Primitive%20Component%20Object%20Reference) (OtherActor :type Actor%20Object%20Reference) (OtherComp :type Primitive%20Component%20Object%20Reference) (OtherBodyIndex :type Integer) (bFromSweep :type Boolean) (SweepResult :type Hit%20Result%20Structure%20%28by%20ref%29))
  (Utilities|Casting|CastToBP_FirstPersonCharacter OtherActor)
  (Variables|/Game/FirstPerson/Blueprints/BP_FirstPersonCharacter.BP_FirstPersonCharacter_C|SetcanSave (Variables|Default|GetplayerCharacter) true)
  (bind _returnvalue (UserInterface|CreateWidget "/Game/Blueprints/UI/BP_SaveGameUI.BP_SaveGameUI_C" (Game|GetPlayerController 0)))
  (Variables|/Game/FirstPerson/Blueprints/BP_FirstPersonCharacter.BP_FirstPersonCharacter_C|SetnearestBall (stale EventBeginPlay _output_get) self)
  (Variables|/Game/FirstPerson/Blueprints/BP_FirstPersonCharacter.BP_FirstPersonCharacter_C|SetsaveWidget (stale EventBeginPlay _output_get) _returnvalue)
  (Variables|Default|SetpauseWidget _returnvalue)
  (UserInterface|Viewport|AddtoViewport _returnvalue 0))

(event OnComponentEndOverlap(CollisionSphere)
  (params (OverlappedComponent :type Primitive%20Component%20Object%20Reference) (OtherActor :type Actor%20Object%20Reference) (OtherComp :type Primitive%20Component%20Object%20Reference) (OtherBodyIndex :type Integer))
  (Utilities|Casting|CastToBP_FirstPersonCharacter OtherActor)
  (Variables|/Game/FirstPerson/Blueprints/BP_FirstPersonCharacter.BP_FirstPersonCharacter_C|SetcanSave (Variables|Default|GetplayerCharacter) false)
  (Widget|RemovefromParent (Variables|Default|GetpauseWidget)))

(event EventBeginPlay
  (bind _returnvalue (Actor|GetActorOfClass "/Game/FirstPerson/Blueprints/BP_FirstPersonCharacter.BP_FirstPersonCharacter_C"))
  (bind _output_get (Variables|Default|SetplayerCharacter _returnvalue)))

(event EventTick
  (params (DeltaSeconds :type Float%20%28single-precision%29))
  (Transformation|AddLocalOffset (Variables|Default|GetSphere) (* (Math|Vector|MakeVector 0.0 0.0 (* (Math|Trig|Sin(Radians) (Actor|GetGameTimeSinceCreation)) 1e+01)) DeltaSeconds) false false))

(fn ConstructionScript
  (Components|Sphere|SetSphereRadius (Variables|Default|GetCollision%20Sphere) (Variables|Default|GetinteractDistance) true))