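; Cerberus is a spinning detector actor with three cone volumes that watch for the first-person player character.
; Tick yaws the whole actor at SpinSpeed scaled by delta time, sweeping the cones around.
; Each cone's begin-overlap casts to BP_FirstPersonCharacter and, if that character's IsDetectable is set, prints its display name.
; Detection triggers nothing beyond that on-screen print.
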(event OnComponentBeginOverlap(Cone)
  (params (OverlappedComponent :type Primitive%20Component%20Object%20Reference) (OtherActor :type Actor%20Object%20Reference) (OtherComp :type Primitive%20Component%20Object%20Reference) (OtherBodyIndex :type Integer) (bFromSweep :type Boolean) (SweepResult :type Hit%20Result%20Structure%20%28by%20ref%29))
  (bind _asbp_first_person_character (Utilities|Casting|CastToBP_FirstPersonCharacter OtherActor))
  (if (Variables|/Game/FirstPerson/Blueprints/BP_FirstPersonCharacter.BP_FirstPersonCharacter_C|GetisDetectable _asbp_first_person_character)
    (Development|PrintString (Utilities|GetDisplayName _asbp_first_person_character) true true "(R=0.000000,G=0.660000,B=1.000000,A=1.000000)" 0.5)))

(event OnComponentBeginOverlap(cone1_0)
  (params (OverlappedComponent :type Primitive%20Component%20Object%20Reference) (OtherActor :type Actor%20Object%20Reference) (OtherComp :type Primitive%20Component%20Object%20Reference) (OtherBodyIndex :type Integer) (bFromSweep :type Boolean) (SweepResult :type Hit%20Result%20Structure%20%28by%20ref%29))
  (bind _asbp_first_person_character (Utilities|Casting|CastToBP_FirstPersonCharacter OtherActor))
  (if (Variables|/Game/FirstPerson/Blueprints/BP_FirstPersonCharacter.BP_FirstPersonCharacter_C|GetisDetectable _asbp_first_person_character)
    (Development|PrintString (Utilities|GetDisplayName _asbp_first_person_character) true true "(R=0.000000,G=0.660000,B=1.000000,A=1.000000)" 0.5)))

(event OnComponentBeginOverlap(cone1_1)
  (params (OverlappedComponent :type Primitive%20Component%20Object%20Reference) (OtherActor :type Actor%20Object%20Reference) (OtherComp :type Primitive%20Component%20Object%20Reference) (OtherBodyIndex :type Integer) (bFromSweep :type Boolean) (SweepResult :type Hit%20Result%20Structure%20%28by%20ref%29))
  (bind _asbp_first_person_character (Utilities|Casting|CastToBP_FirstPersonCharacter OtherActor))
  (if (Variables|/Game/FirstPerson/Blueprints/BP_FirstPersonCharacter.BP_FirstPersonCharacter_C|GetisDetectable _asbp_first_person_character)
    (Development|PrintString (Utilities|GetDisplayName _asbp_first_person_character) true true "(R=0.000000,G=0.660000,B=1.000000,A=1.000000)" 0.5)))

(event EventBeginPlay)

(event Collision|EventActorBeginOverlap
  (params (OtherActor :type Actor%20Object%20Reference)))

(event EventTick
  (params (DeltaSeconds :type Float%20%28single-precision%29))
  (bind _output_get (Variables|Default|SetrotationAmount (* DeltaSeconds (Variables|Default|GetspinSpeed))))
  (Transformation|AddActorLocalRotation (Math|Rotator|MakeRotator 0.0 0.0 _output_get) false false))

(fn ConstructionScript)