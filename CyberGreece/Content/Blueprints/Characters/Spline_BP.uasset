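; Spline path actor in Characters that moves a referenced TargetActor along its spline with the Movement timeline.
; The construction script snaps the target to the first spline point.
; PlayTimeline plays forward or reverses by IsInverse, mapping timeline Coef to spline distance and flipping the flag on finish to ping-pong.
; BeginPlay is empty, and the Duration-based play rate, initial PlayTimeline call and tangent-facing rotation are unwired.
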(event Custom|Play%20Timeline
  (bind _spline (Variables|Default|GetSpline))
  (if (Variables|Default|GetisInverse)
    (bind _coef (Timeline|Movement PlayFromStart)
      (:Update
        (Transformation|SetActorLocation (Variables|Default|GettargetActor) (Spline|GetLocationatDistanceAlongSpline (Variables|Default|GetSpline) (Math|Float|Lerp 0.0 (Spline|GetDistanceAlongSplineatSplinePoint _spline (- (Spline|GetNumberOfSplinePoints _spline) 1)) _coef) "World") false false))
      (:Finished
        (Variables|Default|SetisInverse (not (Variables|Default|GetisInverse)))
        (CallFunction|PlayTimeline)))
    (else
      (Timeline|Movement Reverse))))

(event EventBeginPlay)

(fn ConstructionScript
  (Transformation|SetActorLocation (Variables|Default|GettargetActor) (Spline|GetLocationatSplinePoint (Variables|Default|GetSpline) 0 "World") false false))