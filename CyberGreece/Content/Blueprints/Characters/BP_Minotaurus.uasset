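; BP_Minotaurus is an enemy character that patrols waypoints and chases pawns it sees.
; Patrol uses AIMoveTo through a looping waypoint array, pausing for a random delay at each point.
; PawnSensing triggers pursuit, with a DoOnce gating the speed boost and alert sound.
; A retriggerable five-second delay after the last sighting re-arms the sprint, slows the walk speed and resumes patrol.
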(event OnSeePawn(PawnSensing)
  (params (Pawn :type Pawn%20Object%20Reference))
  (Utilities|FlowControl|Sequence
    (:then_0
      (Utilities|FlowControl|DoOnce false
        (:Completed
          (Variables|/Script/Engine.CharacterMovementComponent|SetMaxWalkSpeed (Variables|Character|GetCharacterMovement) 4e+02)
          (Variables|Default|SetisChasing true)
          (Audio|PlaySoundatLocation "/Game/Audio/alert.alert" (Transformation|GetActorLocation) "0, 0, 0" 1.0 1.0 0.0 0 0 0 0))))
    (:then_1
      (AI|AIMoveTo self "0, 0, 0" Pawn 5.0 false
        (:then
          (Utilities|FlowControl|RetriggerableDelay 5.0)
          (CallFunction|CanSprintAgain)
          (Variables|/Script/Engine.CharacterMovementComponent|SetMaxWalkSpeed (Variables|Character|GetCharacterMovement) 1e+02)
          (CallFunction|MovetoLocation))))))

(event Custom|MoveToLocation
  (Variables|Default|SetisChasing false)
  (AI|AIMoveTo self (Transformation|GetWorldLocation (Variables|/Game/Blueprints/BP_Waypoint.BP_Waypoint_C|GetDefaultSceneRoot (Utilities|Array|Get(acopy) (Variables|Default|Getwaypoints) (Variables|Default|GetwaypointIndex)))) 0 5.0 false
    (:OnSuccess
      (Utilities|FlowControl|Delay (Math|Random|RandomFloatinRange (Variables|Default|GetminDelay) (Variables|Default|GetmaxDelay)))
      (if (not (Variables|Default|GetisChasing))
        (Math|Integer|IncrementInt (Variables|Default|GetwaypointIndex)
          (:%20%20
            (if (>= (Variables|Default|GetwaypointIndex) (Utilities|Array|Length (Variables|Default|Getwaypoints)))
              (Variables|Default|SetwaypointIndex 0)
              (CallFunction|MovetoLocation)
              (else
                (CallFunction|MovetoLocation)))))))))

(event Custom|CanSprintAgain
  (Utilities|FlowControl|DoOnce false) ; enters at Reset
)

(event EventBeginPlay
  (Variables|Default|SetwaypointIndex 0)
  (CallFunction|MovetoLocation))

(fn ConstructionScript)