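; Patrolling statue that watches for the first-person character, currently only printing its name when detected.
; A looping Movement timeline, alternating forward and reverse, slides the body between the spline's first and last points while sweeping its yaw across a turn angle.
; Each tick, ten debug-drawn object traces fan out randomly from the head's forward vector within a set spread, reporting only characters flagged as detectable.
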(event Custom|Move
  (bind _spline (Variables|Default|GetSpline))
  (bind _statue_body (Variables|Default|GetStatue%20Body))
  (bind _turnangle (Variables|Default|GetturnAngle))
  (bind _returnvalue (Transformation|GetWorldRotation _statue_body))
  (if (Variables|Default|GetisFlipped)
    (bind _coef (Timeline|Movement Reverse)
      (:Update
        (Transformation|SetRelativeLocation _statue_body (Spline|GetLocationatDistanceAlongSpline (Variables|Default|GetSpline) (Math|Float|Lerp 0.0 (Spline|GetDistanceAlongSplineatSplinePoint _spline (- (Spline|GetNumberOfSplinePoints _spline) 1)) _coef) "Local") false false)
        (Transformation|SetWorldRotation _statue_body (Math|Rotator|MakeRotator (.roll _returnvalue) (.pitch _returnvalue) (+ (Math|Float|Lerp _turnangle (* _turnangle -1.0) _coef) 1.8e+02)) false false))
      (:Finished
        (Variables|Default|SetisFlipped (not (Variables|Default|GetisFlipped)))
        (CallFunction|Move)))
    (else
      (Timeline|Movement PlayFromStart))))

(event EventBeginPlay
  (Components|Timeline|SetPlayRate (Variables|Default|GetMovement) (/ 1.0 (Variables|Default|GetturnDuration)))
  (CallFunction|Move))

(event EventTick
  (params (DeltaSeconds :type Float%20%28single-precision%29))
  (bind _statue_head (Variables|Default|GetStatue%20Head))
  (bind _spread (Variables|Default|Getspread))
  (bind _spread_2 (Variables|Default|Getspread))
  (bind _spread_3 (Variables|Default|Getspread))
  (bind _returnvalue (Transformation|GetWorldLocation _statue_head))
  (for _index (range 0 9)
    (bind _outhit (Collision|LineTraceForObjects _returnvalue (+ _returnvalue (* (Math|Vector|GetForwardVector _statue_head) (Variables|Default|GetdetectRange)) (Math|Vector|MakeVector (Math|Random|RandomFloatinRange (* _spread -1.0) _spread) (Math|Random|RandomFloatinRange (* _spread_2 -1.0) _spread_2) (Math|Random|RandomFloatinRange (* _spread_3 -1.0) _spread_3))) (Variables|Default|GetObject%20Types) false 0 "ForOneFrame"))
    (bind _asbp_first_person_character (Utilities|Casting|CastToBP_FirstPersonCharacter (.HitActor (Collision|BreakHitResult _outhit))))
    (if (Variables|/Game/FirstPerson/Blueprints/BP_FirstPersonCharacter.BP_FirstPersonCharacter_C|GetisDetectable _asbp_first_person_character)
      (Development|PrintString (Utilities|GetDisplayName _asbp_first_person_character) true true "(R=0.000000,G=0.660000,B=1.000000,A=1.000000)" 0.5))))

(fn ConstructionScript)