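; BP_Minotaurus is an AI enemy that loops through a list of waypoints and chases pawns it sees.
; MoveToLocation runs AI Move To toward the current waypoint, advancing and wrapping the index on each success.
; PawnSensing raises walk speed and redirects movement to the seen pawn.
; A Retriggerable Delay, restarted by each sighting, restores the slower speed and resumes patrol two seconds after the last one.
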(event OnSeePawn(PawnSensing)
  (params (Pawn :type Pawn%20Object%20Reference))
  (Utilities|FlowControl|Sequence
    (:then_0
      (Variables|/Script/Engine.CharacterMovementComponent|SetMaxWalkSpeed (Variables|Character|GetCharacterMovement) 6e+02))
    (:then_1
      (AI|AIMoveTo self "0, 0, 0" Pawn 5.0 false
        (:then
          (Utilities|FlowControl|RetriggerableDelay 2.0)
          (Variables|/Script/Engine.CharacterMovementComponent|SetMaxWalkSpeed (Variables|Character|GetCharacterMovement) 2e+02)
          (CallFunction|MovetoLocation))))))

(event Custom|MoveToLocation
  (AI|AIMoveTo self (Transformation|GetWorldLocation (Variables|/Game/Blueprints/BP_Waypoint.BP_Waypoint_C|GetDefaultSceneRoot (Utilities|Array|Get(acopy) (Variables|Default|Getwaypoints) (Variables|Default|GetwaypointIndex)))) 0 5.0 false
    (:OnSuccess
      (Math|Integer|IncrementInt (Variables|Default|GetwaypointIndex)
        (:%20%20
          (if (>= (Variables|Default|GetwaypointIndex) (Utilities|Array|Length (Variables|Default|Getwaypoints)))
            (Variables|Default|SetwaypointIndex 0)
            (CallFunction|MovetoLocation)
            (else
              (CallFunction|MovetoLocation))))))))

(event EventBeginPlay
  (Variables|Default|SetwaypointIndex 0)
  (CallFunction|MovetoLocation))

(event Collision|EventActorBeginOverlap
  (params (OtherActor :type Actor%20Object%20Reference)))

(event EventTick
  (params (DeltaSeconds :type Float%20%28single-precision%29)))

(fn ConstructionScript)