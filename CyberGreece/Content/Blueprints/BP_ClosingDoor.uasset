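; BP_ClosingDoor is a door that seals behind the first-person player and saves the game.
; The construction script hides the Door and disables its collision.
; When BP_FirstPersonCharacter leaves the Box trigger, the Door becomes visible and solid, then SaveGame is called on the character reference cached at BeginPlay.
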(event OnComponentEndOverlap(Box)
  (params (OverlappedComponent :type Primitive%20Component%20Object%20Reference) (OtherActor :type Actor%20Object%20Reference) (OtherComp :type Primitive%20Component%20Object%20Reference) (OtherBodyIndex :type Integer))
  (Utilities|Casting|CastToBP_FirstPersonCharacter OtherActor)
  (Rendering|SetVisibility (Variables|Default|GetDoor) true false)
  (Collision|SetCollisionEnabled (Variables|Default|GetDoor) "QueryAndPhysics")
  (Default|SaveGame (Variables|Default|GetplayerCharacter)))

(event EventBeginPlay
  (bind _returnvalue (Actor|GetActorOfClass "/Game/FirstPerson/Blueprints/BP_FirstPersonCharacter.BP_FirstPersonCharacter_C"))
  (Variables|Default|SetplayerCharacter _returnvalue))

(fn ConstructionScript
  (Rendering|SetVisibility (Variables|Default|GetDoor) false false)
  (Collision|SetCollisionEnabled (Variables|Default|GetDoor) "NoCollision"))