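; BP_Scroll is an interactable scroll actor that the first-person character can pick up and add to a Table.
; The construction script applies the configurable pickup radius and scroll material.
; While interactable, sphere overlaps show or remove an interact widget and set or clear the character's NearestScroll reference.
; Pickup plays a sound, passes the scroll to Table.AddScroll, disables interaction and removes the widget.
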(event OnComponentBeginOverlap(Sphere)
  (params (OverlappedComponent :type Primitive%20Component%20Object%20Reference) (OtherActor :type Actor%20Object%20Reference) (OtherComp :type Primitive%20Component%20Object%20Reference) (OtherBodyIndex :type Integer) (bFromSweep :type Boolean) (SweepResult :type Hit%20Result%20Structure%20%28by%20ref%29))
  (if (Variables|Default|GetisInteractable)
    (Utilities|Casting|CastToBP_FirstPersonCharacter OtherActor)
    (bind _returnvalue (UserInterface|CreateWidget "/Game/Blueprints/UI/BP_InteractUI.BP_InteractUI_C" (Game|GetPlayerController 0)))
    (bind _output_get (Variables|Default|SetinteractWidget _returnvalue))
    (UserInterface|Viewport|AddtoViewport _output_get 0)
    (Variables|/Game/FirstPerson/Blueprints/BP_FirstPersonCharacter.BP_FirstPersonCharacter_C|SetnearestScroll (Variables|Default|GetplayerCharacter) self)))

(event OnComponentEndOverlap(Sphere)
  (params (OverlappedComponent :type Primitive%20Component%20Object%20Reference) (OtherActor :type Actor%20Object%20Reference) (OtherComp :type Primitive%20Component%20Object%20Reference) (OtherBodyIndex :type Integer))
  (if (Variables|Default|GetisInteractable)
    (Utilities|Casting|CastToBP_FirstPersonCharacter OtherActor)
    (Widget|RemovefromParent (Variables|Default|GetinteractWidget))
    (Variables|/Game/FirstPerson/Blueprints/BP_FirstPersonCharacter.BP_FirstPersonCharacter_C|SetnearestScroll (Variables|Default|GetplayerCharacter) 0)))

(event EventBeginPlay
  (bind _returnvalue (Actor|GetActorOfClass "/Game/FirstPerson/Blueprints/BP_FirstPersonCharacter.BP_FirstPersonCharacter_C"))
  (Variables|Default|SetplayerCharacter _returnvalue))

(event Collision|EventActorBeginOverlap
  (params (OtherActor :type Actor%20Object%20Reference)))

(event EventTick
  (params (DeltaSeconds :type Float%20%28single-precision%29)))

(fn ConstructionScript
  (Components|Sphere|SetSphereRadius (Variables|Default|GetSphere) (Variables|Default|GetpickupRadius) true)
  (Rendering|Material|SetMaterial (Variables|Default|GetScroll%20Model) 1 (Variables|Default|GetscrollMaterial)))

(fn Pickup
  (Audio|PlaySoundatLocation "/Game/Audio/Scroll_pickup_Cue.Scroll_pickup_Cue" (Transformation|GetActorLocation) "0, 0, 0" 1.0 1.0 0.0 0 0 0 0)
  (Development|PrintString "scroll picked")
  (Default|AddScroll (Variables|Default|Gettable) self)
  (Variables|Default|SetisInteractable false)
  (Widget|RemovefromParent (Variables|Default|GetinteractWidget)))