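; Portal trigger actor that teleports the first-person character to a Destination actor when it enters the Box.
; Converts player 0's location into the trigger's local space with X and Y scale negated, then maps it through the Destination's transform.
; Mirrors the rotation axes across local X and Y the same way, so the exit pose keeps its relative offset, turned half a turn about Z.
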(event OnComponentBeginOverlap(Box)
  (params (OverlappedComponent :type Primitive%20Component%20Object%20Reference) (OtherActor :type Actor%20Object%20Reference) (OtherComp :type Primitive%20Component%20Object%20Reference) (OtherBodyIndex :type Integer) (bFromSweep :type Boolean) (SweepResult :type Hit%20Result%20Structure%20%28by%20ref%29))
  (bind _returnvalue (Transformation|GetActorTransform))
  (bind _returnvalue_2 (Game|GetPlayerCharacter 0))
  (bind _returnvalue_3 (Transformation|GetActorTransform))
  (bind _destination (Variables|Default|GetDestination))
  (bind _returnvalue_4 (Transformation|GetActorRotation _returnvalue_2))
  (bind (_location _rotation _scale) (Math|Transform|BreakTransform _returnvalue))
  (bind _returnvalue_5 (Transformation|GetActorTransform _destination))
  (bind (_x _y _z) (Math|Rotator|GetAxes _returnvalue_4))
  (bind _asbp_first_person_character (Utilities|Casting|CastToBP_FirstPersonCharacter OtherActor))
  (Transformation|SetActorTransform _asbp_first_person_character (Math|Transform|MakeTransform (Math|Transform|TransformLocation (Transformation|GetActorTransform (Variables|Default|GetDestination)) (Math|Transform|InverseTransformLocation (Math|Transform|MakeTransform _location _rotation (Math|Vector|MakeVector (* (.x _scale) -1.0) (* (.y _scale) -1.0) (.z _scale))) (Transformation|GetActorLocation (Game|GetPlayerCharacter 0)))) (Math|Rotator|MakeRotationfromAxes (Math|Transform|TransformDirection _returnvalue_5 (Math|Vector|MirrorVectorbyNormal (Math|Vector|MirrorVectorbyNormal (Math|Transform|InverseTransformDirection _returnvalue_3 _x) "1.000000,0.000000,0.000000") "0.000000,1.000000,0.000000")) (Math|Transform|TransformDirection _returnvalue_5 (Math|Vector|MirrorVectorbyNormal (Math|Vector|MirrorVectorbyNormal (Math|Transform|InverseTransformDirection _returnvalue_3 _y) "1.000000,0.000000,0.000000") "0.000000,1.000000,0.000000")) (Math|Transform|TransformDirection _returnvalue_5 (Math|Vector|MirrorVectorbyNormal (Math|Vector|MirrorVectorbyNormal (Math|Transform|InverseTransformDirection _returnvalue_3 _z) "1.000000,0.000000,0.000000") "0.000000,1.000000,0.000000"))) "1.000000,1.000000,1.000000") false true))

(event EventBeginPlay)

(event Collision|EventActorBeginOverlap
  (params (OtherActor :type Actor%20Object%20Reference)))

(event EventTick
  (params (DeltaSeconds :type Float%20%28single-precision%29)))

(fn ConstructionScript)