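; Portal door that toggles the first-person camera's post-process material and swaps its own Entry material each time the player passes through it.
; While the player overlaps PlayerDetection, Tick detects crossings using the camera's side of the Arrow-defined plane and a line-plane intersection from its last position.
; PreventPlaneClipping nudges the Entry away from the camera when it is close to the plane.
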(event EventBeginPlay)

(event Collision|EventActorBeginOverlap
  (params (OtherActor :type Actor%20Object%20Reference)))

(event EventTick
  (params (DeltaSeconds :type Float%20%28single-precision%29))
  (if (Collision|IsOverlappingActor (Variables|Default|GetPlayer%20detection) (Game|GetPlayerCharacter 0) :!class /Script/Engine.PrimitiveComponent)
    (CallFunction|PreventPlaneClipping)
    (bind _iscrossing1 (CallFunction|HasCrossedDoor))
    (if _iscrossing1
      (if (Variables|Default|GetisInverted)
        (Variables|Default|SetisInverted false)
        (Rendering|Material|SetMaterial (Variables|Default|GetEntry) 0 (Variables|Default|GetDoorMaterial))
        (Variables|/Script/Engine.CameraComponent|SetPostProcessSettings (Variables|/Game/FirstPerson/Blueprints/BP_FirstPersonCharacter.BP_FirstPersonCharacter_C|GetFirstPersonCamera (.AsBP%20First%20Person%20Character (Utilities|Casting|CastToBP_FirstPersonCharacter (Game|GetPlayerCharacter 0)))) (Utilities|Struct|MakePostProcessSettings (Utilities|Struct|MakeWeightedBlendables (Utilities|Array|MakeArray (Utilities|Struct|MakeWeightedBlendable 1.0 "/Game/Portals/Materials/Default_Shader_PPM.Default_Shader_PPM")))))
        (else
          (Variables|Default|SetisInverted true)
          (Rendering|Material|SetMaterial (Variables|Default|GetEntry) 0 "/Game/Portals/Materials/Default_Shader.Default_Shader")
          (Variables|/Script/Engine.CameraComponent|SetPostProcessSettings (Variables|/Game/FirstPerson/Blueprints/BP_FirstPersonCharacter.BP_FirstPersonCharacter_C|GetFirstPersonCamera (.AsBP%20First%20Person%20Character (Utilities|Casting|CastToBP_FirstPersonCharacter (Game|GetPlayerCharacter 0)))) (Utilities|Struct|MakePostProcessSettings (Utilities|Struct|MakeWeightedBlendables (Utilities|Array|MakeArray (Utilities|Struct|MakeWeightedBlendable 1.0 (Variables|Default|GetpostProcessMaterial)))))))))
    (else
      (Variables|Default|SetisOverlapping false))))

(fn ConstructionScript
  (Rendering|Material|SetMaterial (Variables|Default|GetEntry) 0 (Variables|Default|GetDoorMaterial)))

(fn HasCrossedDoor
  (LocalVariables|SetisInFront (>= (Math|Vector|DotProduct (Math|Vector|GetForwardVector (Variables|Default|GetArrow)) (- (Transformation|GetWorldLocation (Variables|/Game/FirstPerson/Blueprints/BP_FirstPersonCharacter.BP_FirstPersonCharacter_C|GetFirstPersonCamera (.AsBP%20First%20Person%20Character (Utilities|Casting|CastToBP_FirstPersonCharacter (Game|GetPlayerCharacter 0))))) (Transformation|GetActorLocation))) 0.0))
  (bind _output_get (LocalVariables|Setplane (Class|KismetMathLibrary|MakePlanefromPointandNormal (Transformation|GetActorLocation) (Math|Vector|GetForwardVector (Variables|Default|GetArrow)))))
  (LocalVariables|SetisIntersecting (.ReturnValue (Class|KismetMathLibrary|LinePlaneIntersection (Transformation|GetWorldLocation (Variables|/Game/FirstPerson/Blueprints/BP_FirstPersonCharacter.BP_FirstPersonCharacter_C|GetFirstPersonCamera (.AsBP%20First%20Person%20Character (Utilities|Casting|CastToBP_FirstPersonCharacter (Game|GetPlayerCharacter 0))))) (Variables|Default|GetlastPosition) _output_get)))
  (LocalVariables|SetisCrossing (or (Math|Boolean|ANDBoolean (LocalVariables|GetisIntersecting) (not (LocalVariables|GetisInFront)) (Variables|Default|GetlastInFront) (Variables|Default|GetisOverlapping)) (Math|Boolean|ANDBoolean (LocalVariables|GetisIntersecting) (LocalVariables|GetisInFront) (not (Variables|Default|GetlastInFront)) (Variables|Default|GetisOverlapping))))
  (Variables|Default|SetlastInFront (LocalVariables|GetisInFront))
  (Variables|Default|SetlastPosition (Transformation|GetWorldLocation (Variables|/Game/FirstPerson/Blueprints/BP_FirstPersonCharacter.BP_FirstPersonCharacter_C|GetFirstPersonCamera (.AsBP%20First%20Person%20Character (Utilities|Casting|CastToBP_FirstPersonCharacter (Game|GetPlayerCharacter 0))))))
  (Variables|Default|SetisOverlapping true)
  (return (LocalVariables|GetisCrossing)))

(fn PreventPlaneClipping
  (bind _returnvalue (Game|GetPlayerCharacter 0))
  (bind _returnvalue_2 (Transformation|GetActorLocation))
  (bind _arrow (Variables|Default|GetArrow))
  (bind _returnvalue_3 (Math|Vector|GetForwardVector _arrow))
  (bind _asbp_first_person_character (Utilities|Casting|CastToBP_FirstPersonCharacter _returnvalue))
  (bind _firstpersoncamera (Variables|/Game/FirstPerson/Blueprints/BP_FirstPersonCharacter.BP_FirstPersonCharacter_C|GetFirstPersonCamera _asbp_first_person_character))
  (bind _returnvalue_4 (Transformation|GetWorldLocation _firstpersoncamera))
  (bind _returnvalue_5 (- _returnvalue_4 _returnvalue_2))
  (bind _returnvalue_6 (Math|Vector|DotProduct _returnvalue_3 _returnvalue_5))
  (if (and (>= _returnvalue_6 -3.0) (<= _returnvalue_6 0.0))
    (Transformation|SetRelativeLocation (Variables|Default|GetEntry) "2.000000,0.000000,0.000000" false false)
    (elif (and (>= _returnvalue_6 -3.0) (<= _returnvalue_6 3.0))
      (Transformation|SetRelativeLocation (Variables|Default|GetEntry) "-2.000000,0.000000,0.000000" false false)
      (else
        (Transformation|SetRelativeLocation (Variables|Default|GetEntry) "0.000000,0.000000,0.000000" false false)))))